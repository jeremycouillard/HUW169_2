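; EnemyBP is an enemy actor with separate overlap volumes for being defeated by the player and for hurting the player.
; Overlapping DamageEnemy spawns a coin particle and destroys the enemy.
; Overlapping DamagePlayer reduces PlayerHealth and briefly pauses all Level Sequence actors so the enemy does not run into the player and kill itself.
; At zero health it disables player movement, shows the Youdied widget and restarts the level after a delay.
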(event `self.damageEnemy.OnComponentBeginOverlap`
  (params (OverlappedComponent :type "PrimitiveComponent Object Reference") (OtherActor :type "Actor Object Reference") (OtherComp :type "PrimitiveComponent Object Reference") (OtherBodyIndex :type Integer) (bFromSweep :type Boolean) (SweepResult :type "HitResult Structure (by ref)"))
  ;[0.2045 0.4034 1] player hits the enemey
  (cast `/Game/PlayerOne/PlayerOne` OtherActor)
  (`GameplayStatics.SpawnEmitterAtLocation` "/Game/getCoinParticle.getCoinParticle" (`self.K2_GetActorLocation`))
  (`self.K2_DestroyActor`))

(event `self.damagePlayer.OnComponentBeginOverlap`
  (params (OverlappedComponent :type "PrimitiveComponent Object Reference") (OtherActor :type "Actor Object Reference") (OtherComp :type "PrimitiveComponent Object Reference") (OtherBodyIndex :type Integer) (bFromSweep :type Boolean) (SweepResult :type "HitResult Structure (by ref)"))
  ;[1 0.09911 0] player gets hit
  ;;[1 1 1] subtracting from the health. The widget picks up this info in a bind function
  (bind _asplayer_one (cast `/Game/PlayerOne/PlayerOne` OtherActor))
  (bind _output_get (set `/Game/PlayerOne/PlayerOne.playerHealth` (- (`/Game/PlayerOne/PlayerOne.playerHealth` _asplayer_one) 0.1) _asplayer_one))
  ;[1 1 1] this will pause the sequence for .2 sec so that the enemy doesn't kill itself by running into the player
  (bind _outactors (`GameplayStatics.GetAllActorsOfClass` "/Script/LevelSequence.LevelSequenceActor"))
  (for _array_element _outactors
    (`LevelSequencePlayer.Pause` (`LevelSequenceActor.SequencePlayer` _array_element)))
  (`KismetSystemLibrary.Delay` 0.5)
  (bind _outactors_2 (`GameplayStatics.GetAllActorsOfClass` "/Script/LevelSequence.LevelSequenceActor"))
  (for _array_element_2 _outactors_2
    (`LevelSequencePlayer.Play` (`LevelSequenceActor.SequencePlayer` _array_element_2)))
  ;;[1 1 1] check if the player is dead - if so pause for a sec and then restart the level
  (if (<= _output_get 0.0)
    (set `/Game/PlayerOne/PlayerOne.canMove?` false _asplayer_one)
    (bind _returnvalue (`|CreateWidget` "/Game/widgets/youdied.youdied_C"))
    (`UserWidget.AddToViewport` _returnvalue 0)
    (`KismetSystemLibrary.Delay` 2.0)
    (`KismetSystemLibrary.ExecuteConsoleCommand` "RestartLevel")))

(fn `UserConstructionScript`)