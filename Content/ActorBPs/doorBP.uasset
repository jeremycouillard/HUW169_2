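; Door actor that gates progression to LevelTwo behind the player's key.
; BeginPlay creates a KeyInfoWidget; a box overlap checks PlayerOne's HasKey and shows a proceed or need-key message.
; With the key, if the widget is not already visible, it waits briefly, disables player movement and opens the level.
; Leaving the box removes the widget.
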(event `self.ReceiveBeginPlay`
  ;[1 1 1] make a widget variable
  (bind _returnvalue (`|CreateWidget` "/Game/widgets/keyInfoWidget.keyInfoWidget_C"))
  (set `self.keyTextWidgetREF` _returnvalue))

(event `self.Box.OnComponentBeginOverlap`
  (params (OverlappedComponent :type "PrimitiveComponent Object Reference") (OtherActor :type "Actor Object Reference") (OtherComp :type "PrimitiveComponent Object Reference") (OtherBodyIndex :type Integer) (bFromSweep :type Boolean) (SweepResult :type "HitResult Structure (by ref)"))
  (bind _keytextwidgetref (`self.keyTextWidgetREF`))
  (bind _keytextwidgetref_2 (`self.keyTextWidgetREF`))
  (bind _asplayer_one (cast `/Game/PlayerOne/PlayerOne` OtherActor))
  (if (`/Game/PlayerOne/PlayerOne.hasKey?` _asplayer_one)
    ;[1 1 1] has the key
    (`TextBlock.SetText` (`/Game/widgets/keyInfoWidget.keyText` (`self.keyTextWidgetREF`)) "You may proceed")
    (if (not (`Widget.IsVisible` _keytextwidgetref))
      (`UserWidget.AddToViewport` _keytextwidgetref 0)
      (`KismetSystemLibrary.Delay` 2.0)
      (set `/Game/PlayerOne/PlayerOne.canMove?` false _asplayer_one)
      (`GameplayStatics.OpenLevel` "LevelTwo"))
    (else
      ;[1 1 1] does not have the key
      (`TextBlock.SetText` (`/Game/widgets/keyInfoWidget.keyText` (`self.keyTextWidgetREF`)) "You need the key!")
      (if (not (`Widget.IsVisible` _keytextwidgetref_2))
        (`UserWidget.AddToViewport` _keytextwidgetref_2 0)))))

(event `self.Box.OnComponentEndOverlap`
  (params (OverlappedComponent :type "PrimitiveComponent Object Reference") (OtherActor :type "Actor Object Reference") (OtherComp :type "PrimitiveComponent Object Reference") (OtherBodyIndex :type Integer))
  (bind _keytextwidgetref (`self.keyTextWidgetREF`))
  ;[1 1 1] take away widget when player isn't at door anymore
  (cast `/Game/PlayerOne/PlayerOne` OtherActor)
  (if (`Widget.IsVisible` _keytextwidgetref)
    (`Widget.RemoveFromParent` _keytextwidgetref)))

(fn `UserConstructionScript`)