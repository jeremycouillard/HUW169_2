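; badThing is a hazard actor that hurts the player on contact.
; When its Collision component overlaps a PlayerOne, it plays a sound and lowers PlayerHealth by a fixed amount, which a widget displays through a binding.
; At zero health it disables the player's movement, shows the Youdied widget and restarts the level by console command after a short delay.
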(event `self.collision.OnComponentBeginOverlap`
  (params (OverlappedComponent :type "PrimitiveComponent Object Reference") (OtherActor :type "Actor Object Reference") (OtherComp :type "PrimitiveComponent Object Reference") (OtherBodyIndex :type Integer) (bFromSweep :type Boolean) (SweepResult :type "HitResult Structure (by ref)"))
  (bind _asplayer_one (cast `/Game/PlayerOne/PlayerOne` OtherActor))
  (`GameplayStatics.PlaySound2D` "/Game/sounds/key1.key1")
  ;[1 1 1] subtracting from the health. The widget picks up this info in a bind function
  (bind _output_get (set `/Game/PlayerOne/PlayerOne.playerHealth` (- (`/Game/PlayerOne/PlayerOne.playerHealth` _asplayer_one) 0.1) _asplayer_one))
  ;[1 1 1] check if the player is dead - if so pause for a sec and then restart the level
  (if (<= _output_get 0.0)
    (set `/Game/PlayerOne/PlayerOne.canMove?` false _asplayer_one)
    (bind _returnvalue (`|CreateWidget` "/Game/widgets/youdied.youdied_C"))
    (`UserWidget.AddToViewport` _returnvalue 0)
    (`KismetSystemLibrary.Delay` 2.0)
    (`KismetSystemLibrary.ExecuteConsoleCommand` "RestartLevel")))

(fn `UserConstructionScript`)